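; Master projectile Blueprint that plays muzzle and impact Niagara effects, in the EnergyBlade effects folder.
; It spawns the muzzle effect at its offset location shortly after BeginPlay.
; When its collision overlaps a BlockingVolume, it stops movement, spawns the hit effect and sets the Niagara "Kill" variable.
; It then destroys itself after a configurable delay.
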(event OnComponentBeginOverlap(VFXCollision)
  (params (OverlappedComponent :type Primitive%20Component%20Object%20Reference) (OtherActor :type Actor%20Object%20Reference) (OtherComp :type Primitive%20Component%20Object%20Reference) (OtherBodyIndex :type Integer) (bFromSweep :type Boolean) (SweepResult :type Hit%20Result%20Structure%20%28by%20ref%29))
  (Utilities|Casting|CastToBlockingVolume OtherActor)
  (Components|Movement|StopMovementImmediately (Variables|Default|GetProjectileMovement))
  (CallFunction|SpawnVFX (Variables|Default|GetHitImpactVFX) (Variables|Default|GetVFX%20Offset))
  (Class|NiagaraComponent|SetVariableBool (Variables|Default|GetNiagaraComponent) "Kill" true)
  (Utilities|FlowControl|Delay (Variables|Default|GetVFXDestoyDelay))
  (Actor|DestroyActor))

(event EventBeginPlay
  (Utilities|FlowControl|Delay 0.01)
  (CallFunction|SpawnVFX (Variables|Default|GetMuzzleVFX) (Variables|Default|GetVFX%20Offset)))

(fn ConstructionScript)

(fn SpawnVFX
  (params (VFX%20to%20spawn :type Niagara%20System%20Object%20Reference) (Offset :type Vector))
  (Utilities|IsValid VFX%20to%20spawn
    (:Is%20Valid
      (Niagara|SpawnSystematLocation VFX%20to%20spawn (+ (Transformation|GetActorLocation) Offset)))))