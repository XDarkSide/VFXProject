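; BP_ProjectileSpawner is a spawner actor that repeatedly fires BP_ProjectileMaster projectiles to play an energy blade VFX.
; On BeginPlay it spawns one immediately, then repeats on a looping timer set by EventCallGap.
; Each projectile spawns at the spawner's transform and receives its muzzle and hit effects, scaled velocity and VFX offset.
; Only the effect assignment sits behind the validity check.
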(event Custom|SpawnProjectileMaster
  (bind _returnvalue (Game|SpawnActorfromClass "/Game/Niagara/22-EnergyBlade/BP_ProjectileMaster.BP_ProjectileMaster_C" (Transformation|GetActorTransform) "Undefined" "MultiplyWithRoot" 0 0))
  (Utilities|FlowControl|Sequence
    (:then_0
      (Utilities|IsValid _returnvalue
        (:Is%20Valid
          (Variables|Default|SetSpawnedVFX _returnvalue)
          (Variables|/Game/Niagara/22-EnergyBlade/BP_ProjectileMaster.BP_ProjectileMaster_C|SetMuzzleVFX (Variables|Default|GetSpawnedVFX) (Variables|Default|GetMuzzle))
          (Variables|/Game/Niagara/22-EnergyBlade/BP_ProjectileMaster.BP_ProjectileMaster_C|SetHitImpactVFX (Variables|Default|GetSpawnedVFX) (Variables|Default|GetHit)))))
    (:then_1
      (Variables|/Script/Engine.MovementComponent|SetVelocity (Variables|/Game/Niagara/22-EnergyBlade/BP_ProjectileMaster.BP_ProjectileMaster_C|GetProjectileMovement (Variables|Default|GetSpawnedVFX)) (* (Variables|Default|GetVelocity) (Variables|Default|GetSpeed))))
    (:then_2
      (Variables|/Game/Niagara/22-EnergyBlade/BP_ProjectileMaster.BP_ProjectileMaster_C|SetVFX%20Offset (Variables|Default|GetSpawnedVFX) (Variables|Default|GetOffset)))))

(event EventBeginPlay
  (CallFunction|SpawnProjectileMaster)
  (Utilities|Time|SetTimerbyEvent (delegate Custom|SpawnProjectileMaster) (Variables|Default|GetEventCallGap) true))

(fn ConstructionScript)