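; BP_SKSampler is a Blueprint that dissolves a skeletal mesh character with an attached Niagara effect when key 1 is pressed.
; DisolveCharacter creates dynamic instances of two material slots, while a timeline drives their dissolve parameter.
; It then attaches the NS_SampleSkeletalbyBP system to the mesh.
; Both SetMaterial calls target slot 0, so the second instance replaces the first there.
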(event Custom|DisolveCharacter
  (Utilities|FlowControl|Sequence
    (:then_0
      (bind _returnvalue (Rendering|Material|CreateDynamicMaterialInstance (Variables|Default|GetSkeletalMesh) 0 0 "None" :!class /Script/Engine.PrimitiveComponent))
      (Variables|Default|SetCreated_Dyn_MI_1 _returnvalue)
      (bind _returnvalue_2 (Rendering|Material|CreateDynamicMaterialInstance (Variables|Default|GetSkeletalMesh) 1 0 "None" :!class /Script/Engine.PrimitiveComponent))
      (Variables|Default|SetCreated_Dyn_MI_2 _returnvalue_2))
    (:then_1
      (Rendering|Material|SetMaterial (Variables|Default|GetSkeletalMesh) 0 (Variables|Default|GetCreated_Dyn_MI_1))
      (Rendering|Material|SetMaterial (Variables|Default|GetSkeletalMesh) 0 (Variables|Default|GetCreated_Dyn_MI_2)))
    (:then_2
      (bind _changevisibility (Timeline|ChangeVisibility Play)
        (:Update
          (Variables|Default|SetChange%20Visibility _changevisibility)
          (Rendering|Material|SetScalarParameterValue (Variables|Default|GetCreated_Dyn_MI_1) "DissolveAmmount" (Variables|Default|GetChange%20Visibility) :!class /Script/Engine.MaterialInstanceDynamic)
          (Rendering|Material|SetScalarParameterValue (Variables|Default|GetCreated_Dyn_MI_2) "DissolveAmmount" (Variables|Default|GetChange%20Visibility) :!class /Script/Engine.MaterialInstanceDynamic))))
    (:then_3
      (Niagara|SpawnSystemAttached "/Game/Niagara/33-SampleSKByBP/NS_SampleSkeletalbyBP.NS_SampleSkeletalbyBP" (Variables|Default|GetSkeletalMesh) "None" "0, 0, 0" "0, 0, 0" "SnapToTarget" false))))

(event EventBeginPlay
  (Input|EnableInput (Game|GetPlayerController 0)))

(event Input|KeyboardEvents|1
  (params (Key :type Key%20Structure :default "None"))
  (:Pressed
    (CallFunction|DisolveCharacter)))

(fn ConstructionScript)