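; BP_MaterialBaker is an editor utility Blueprint that bakes a material into a static 2D texture asset.
; BakeMaterial checks that the source material and target render target are valid, draws the material into the render target, then saves it as a named texture through an editor-only call.
; It prints a debug message afterwards, and its event graph and construction script do nothing.
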(event EventBeginPlay)

(event Collision|EventActorBeginOverlap
  (params (OtherActor :type Actor%20Object%20Reference)))

(event EventTick
  (params (DeltaSeconds :type Float%20%28single-precision%29)))

(fn ConstructionScript)

(fn BakeMaterial
  (if (and (Utilities|IsValid (Variables|Default|GetTo_RT)) (Utilities|IsValid (Variables|Default|GetFrom_MI)))
    (Rendering|DrawMaterialtoRenderTarget (Variables|Default|GetTo_RT) (Variables|Default|GetFrom_MI))
    (Class|KismetRenderingLibrary|RenderTargetCreateStaticTexture2DEditorOnly (Variables|Default|GetTo_RT) (Variables|Default|GetName) "TC_Default" "TMGS_FromTextureGroup")
    (Development|PrintString "Hello")))